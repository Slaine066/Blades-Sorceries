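; BP_Mage is a mage player character that relays its gameplay events to the player's UI through BP_PlayerController.
; BeginPlay pushes initial health and experience, then binds dispatchers for damage, healing, item and experience pickups, and level-up selection.
; Handlers refresh the matching UI, with hits also spawning floating damage numbers.
; Selection end notifies the controller, but the selection-start handler is empty and its UI update is disconnected.
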(event Custom|OnPickUpExp_Event
  (bind _attributes (Variables|Default|GetAttributes))
  ;[1 1 1] Update Player Get Exp
  (bind _asbp_player_controller (Utilities|Casting|CastToBP_PlayerController (Pawn|GetController)))
  (Default|UpdatePlayerExpInfo _asbp_player_controller (.experiencemax _attributes) (.experience _attributes) (.level _attributes)))

(event Custom|OnLevelUpItemSelectionEnd_Event
  (bind _asbp_player_controller (Utilities|Casting|CastToBP_PlayerController (Pawn|GetController)))
  (Default|EndLevelupItemSelection _asbp_player_controller))

(event Custom|OnHitDamage_Event
  (params (iDamage :type Integer))
  (bind _attributes (Variables|Default|GetAttributes))
  ;[1 1 1] Update Player Hit Damage UI
  (Game|SpawnActorfromClass "/Game/Portfolio_0/UI/FloatingDamage/BP_DamageNumbersActor.BP_DamageNumbersActor_C" (Math|Transform|MakeTransform (+ (Transformation|GetActorLocation) (Variables|Default|GetLocationOffset)) "0, 0, 0" "1.000000,1.000000,1.000000") "Undefined" "MultiplyWithRoot" 0 iDamage (Variables|Default|GetHitDamageColorRGBA) (Variables|Default|GetFontSize) (Variables|Default|GetOutlineSize) 0)
  (bind _asbp_player_controller (Utilities|Casting|CastToBP_PlayerController (Pawn|GetController)))
  (Default|UpdatePlayScreenInfo _asbp_player_controller (.healthmax _attributes) (.health _attributes)))

(event Custom|OnIncreaseHealth_Event
  (bind _attributes (Variables|Default|GetAttributes))
  (bind _asbp_player_controller (Utilities|Casting|CastToBP_PlayerController (Pawn|GetController)))
  (Default|UpdatePlayScreenInfo _asbp_player_controller (.healthmax _attributes) (.health _attributes)))

(event Custom|OnLevelUpItemSelection_Event_0
  (params (ChoiceItemArray :type Array%20of%20Item%20Data%20Structures)))

(event Custom|OnPickUpItem_Event
  (params (InventoryArray :type Array%20of%20Item%20Base%20Object%20References))
  ;[1 1 1] Update PIckup Item Slot
  (bind _asbp_player_controller (Utilities|Casting|CastToBP_PlayerController (Pawn|GetController)))
  (Default|UpdateItemSlotInfo _asbp_player_controller InventoryArray))

(event EventBeginPlay
  (bind _attributes (Variables|Default|GetAttributes))
  (bind _asbp_player_controller (Utilities|Casting|CastToBP_PlayerController (Pawn|GetController)))
  (Default|UpdatePlayScreenInfo _asbp_player_controller (.healthmax _attributes) (.health _attributes))
  (Default|UpdatePlayerExpInfo _asbp_player_controller (.experiencemax _attributes) (.experience _attributes) (.level _attributes))
  ;[1 1 1] Update Player Hit Damage UI
  (EventDispatchers|AssignOnHitDamage (delegate Custom|OnHitDamage_Event))
  (EventDispatchers|AssignOnIncreaseHealth (delegate Custom|OnIncreaseHealth_Event))
  ;[1 1 1] Update PIckup Item Slot
  (EventDispatchers|AssignOnPickUpItem (delegate Custom|OnPickUpItem_Event))
  ;[1 1 1] Update Player Get Exp
  (EventDispatchers|AssignOnPickUpExp (delegate Custom|OnPickUpExp_Event))
  (EventDispatchers|AssignOnLevelUpItemSelection (delegate Custom|OnLevelUpItemSelection_Event_0))
  (EventDispatchers|AssignOnLevelUpItemSelectionEnd (delegate Custom|OnLevelUpItemSelectionEnd_Event)))

(fn ConstructionScript)