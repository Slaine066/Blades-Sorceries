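; BP_GameStateCustom is a game state Blueprint that relays game time and stage number to BP_PlayerController.
; On BeginPlay it binds handlers to the OnGetTime and OnGetMonsterCount dispatchers.
; The time handler updates the first player controller's clock and derives the stage number as minutes plus one.
; The monster count handler only casts the controller, as its UpdateMobCount call is disconnected.
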(event Custom|OnGetMonsterCount_Event
  (params (MobCount :type Integer))
  (bind _asbp_player_controller (Utilities|Casting|CastToBP_PlayerController (Game|GetPlayerController 0))))

(event Custom|OnGetTime_Event
  (params (Minutes :type Integer) (Seconds :type Integer))
  (bind _asbp_player_controller (Utilities|Casting|CastToBP_PlayerController (Game|GetPlayerController 0)))
  (Default|UpdateStageNum _asbp_player_controller (+ Minutes 1))
  (Default|UpdateGameTime _asbp_player_controller Minutes Seconds))

(event EventBeginPlay
  (EventDispatchers|AssignOnGetTime (delegate Custom|OnGetTime_Event))
  (EventDispatchers|AssignOnGetMonsterCount (delegate Custom|OnGetMonsterCount_Event)))

(fn ConstructionScript)