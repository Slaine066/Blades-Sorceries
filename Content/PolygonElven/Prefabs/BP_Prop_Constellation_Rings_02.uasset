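; Animated constellation rings prop from the PolygonElven pack, built from a stand and three ring meshes.
; On BeginPlay, four RotatingMovement components are each assigned one mesh as their updated component, so the stand and each ring rotate independently.
; The construction script is empty, and a leftover AddLocalRotation node is never executed.
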(event EventBeginPlay
  (Components|Movement|SetUpdatedComponent (Variables|Default|GetRotatingMovement) (Variables|Default|GetSM_Prop_Constellation_Rings_01_Stand_01))
  (Components|Movement|SetUpdatedComponent (Variables|Default|GetRotatingMovement1) (Variables|Default|GetSM_Prop_Constellation_Rings_01_Ring_01))
  (Components|Movement|SetUpdatedComponent (Variables|Default|GetRotatingMovement2) (Variables|Default|GetSM_Prop_Constellation_Rings_01_Ring_02))
  (Components|Movement|SetUpdatedComponent (Variables|Default|GetRotatingMovement3) (Variables|Default|GetSM_Prop_Constellation_Rings_01_Ring_03)))

(fn ConstructionScript)