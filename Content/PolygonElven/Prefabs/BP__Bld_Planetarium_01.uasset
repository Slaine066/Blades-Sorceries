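; Animated planetarium building prop from the PolygonElven set, with a rotating middle piece, rings, gears and planets.
; On BeginPlay, each of fourteen RotatingMovement components is retargeted with SetUpdatedComponent to its own static mesh part, so the parts spin independently without Tick logic.
; The graph sets no rotation values, and the construction script is empty.
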(event EventBeginPlay
  (Components|Movement|SetUpdatedComponent (Variables|Default|GetRotatingMovement) (Variables|Default|GetSM_Bld_Planetarium_01_Middle))
  (Components|Movement|SetUpdatedComponent (Variables|Default|GetRotatingMovement1) (Variables|Default|GetSM_Bld_Planetarium_01_Ring_02))
  (Components|Movement|SetUpdatedComponent (Variables|Default|GetRotatingMovement2) (Variables|Default|GetSM_Bld_Planetarium_01_Ring_03))
  (Components|Movement|SetUpdatedComponent (Variables|Default|GetRotatingMovement3) (Variables|Default|GetSM_Bld_Planetarium_01_Ring_04))
  (Components|Movement|SetUpdatedComponent (Variables|Default|GetRotatingMovement4) (Variables|Default|GetSM_Bld_Planetarium_01_Gear_02))
  (Components|Movement|SetUpdatedComponent (Variables|Default|GetRotatingMovement5) (Variables|Default|GetSM_Bld_Planetarium_01_Gear_03))
  (Components|Movement|SetUpdatedComponent (Variables|Default|GetRotatingMovement6) (Variables|Default|GetSM_Bld_Planetarium_01_Gear_04))
  (Components|Movement|SetUpdatedComponent (Variables|Default|GetRotatingMovement7) (Variables|Default|GetSM_Bld_Planetarium_01_Gear_05))
  (Components|Movement|SetUpdatedComponent (Variables|Default|GetRotatingMovement8) (Variables|Default|GetSM_Bld_Planetarium_01_Gear_06))
  (Components|Movement|SetUpdatedComponent (Variables|Default|GetRotatingMovement9) (Variables|Default|GetSM_Bld_Planetarium_01_Gear_07))
  (Components|Movement|SetUpdatedComponent (Variables|Default|GetRotatingMovement10) (Variables|Default|GetSM_Bld_Planetarium_01_ring01_Planet_01))
  (Components|Movement|SetUpdatedComponent (Variables|Default|GetRotatingMovement11) (Variables|Default|GetSM_Bld_Planetarium_01_ring01_Planet_03))
  (Components|Movement|SetUpdatedComponent (Variables|Default|GetRotatingMovement12) (Variables|Default|GetSM_Bld_Planetarium_01_ring01_Planet_01_1))
  (Components|Movement|SetUpdatedComponent (Variables|Default|GetRotatingMovement13) (Variables|Default|GetSM_Bld_Planetarium_01_ring01_Planet_02_1)))

(fn ConstructionScript)